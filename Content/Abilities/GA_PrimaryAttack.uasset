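; GA_PrimaryAttack is a Gameplay Ability for a melee attack that commits, plays a one-handed combat montage and ends when it completes.
; On the authority, it waits DelayHitDetect, then takes a one-off overlap check of the avatar's MeleeStrikeDetector.
; Each other CharacterBase found gets GE_Damage_Melee_Base applied by the attacker's ability system, though the spec and context come from the target's.
; Debug prints report hits and invalid ability systems.
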(event `self.K2_ActivateAbility`
  (bind _returnvalue (`self.K2_CommitAbility`))
  (if _returnvalue
    (`AbilityTask_PlayMontageAndWait.CreatePlayMontageAndWaitProxy` "MeleeAttackAnim" "/Game/Blink/Characters/LowPoly/Humans/Male/Anims/LP_AM_Male_Combat_1H.LP_AM_Male_Combat_1H" 1.0 "None" true 1.0 0.0 true
      (:`then`
        (`self.K2_HasAuthority`
          (:`True`
            (`KismetSystemLibrary.Delay` (`self.DelayHitDetect`))
            (bind _ascharacter_base (cast `CharacterBase` (`self.GetAvatarActorFromActorInfo`)))
            (for _array_element (`PrimitiveComponent.GetOverlappingActors` (`CharacterBase.MeleeStrikeDetector` _ascharacter_base) "/Script/TalesDungeoneer.CharacterBase")
              (if (!= _array_element _ascharacter_base)
                (`|ExecutionSequence`
                  (:`then_0`
                    (`KismetSystemLibrary.PrintString` (`KismetStringLibrary.Concat_StrStr` "Hit '" (`KismetSystemLibrary.GetDisplayName` _array_element) "'")))
                  (:`then_1`
                    (bind _returnvalue_2 (`AbilitySystemBlueprintLibrary.GetAbilitySystemComponent` _array_element))
                    (if (`KismetSystemLibrary.IsValid` _returnvalue_2)
                      (`AbilitySystemComponent.BP_ApplyGameplayEffectSpecToTarget` (`AbilitySystemBlueprintLibrary.GetAbilitySystemComponent` _ascharacter_base) (`AbilitySystemComponent.MakeOutgoingSpec` _returnvalue_2 "/RoleStats/Effects/GE_Damage_Melee_Base.GE_Damage_Melee_Base_C" 1.0 (`AbilitySystemComponent.MakeEffectContext` _returnvalue_2)) _returnvalue_2)
                      (else
                        (`KismetSystemLibrary.PrintString` "Hit Failed - Invalid Ability System" true true (struct :`R` 1.0 :`G` 0.13276 :`A` 1.0) 5.0))))))))))
      (:`OnCompleted`
        (`self.K2_EndAbility`)))
    (else
      (`self.K2_EndAbility`))))